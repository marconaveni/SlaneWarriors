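; Elvenlin player character Blueprint with sprite visuals, damage reaction and switching to BP_Hunter.
; Horizontal movement past a speed threshold reports facing to BP_CameraAdvanced when not attacking.
; Damage, gated by a DoOnce, launches the character by hit direction, disables input and swaps collision profile while a timeline tints the sprite.
; ChangePlayer possesses the Hunter and retargets the camera; landing sets a smoke particle.
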(event `InputAxis|MoveRight` :overrideparent false
  (params (AxisValue :type "Float (single-precision)"))
  (bind _velocity_x (`KismetMathLibrary.BreakVector` (`MovementComponent.Velocity` (`self.CharacterMovement`))))
  (bind _velocity_x_2 (`KismetMathLibrary.BreakVector` (`MovementComponent.Velocity` (`self.CharacterMovement`))))
  ;[1 0.1765 0.1451] Handle movement
  (if (not (`self.isAttackElvenlin`))
    (`/Engine/EditorBlueprintResources/StandardMacros.CompareFloat` AxisValue
      (:`>`
        (if (> _velocity_x_2 200.0)
          (bind _returnvalue (`GameplayStatics.GetActorOfClass` "/Game/Camera/BP_CameraAdvanced.BP_CameraAdvanced_C"))
          (message `/Game/Interfaces/I_Camera.DirectionActor` _returnvalue (`self.isMoveRightElvenlin`))))
      (:`<`
        (if (< _velocity_x -200.0)
          (bind _returnvalue_2 (`GameplayStatics.GetActorOfClass` "/Game/Camera/BP_CameraAdvanced.BP_CameraAdvanced_C"))
          (message `/Game/Interfaces/I_Camera.DirectionActor` _returnvalue_2 (`self.isMoveRightElvenlin`)))))))

(event `InteractInterface.ApplyDamage`
  (params (ActorLocation :type "Vector Structure") (Value :type "Float (single-precision)"))
  (bind (_returnvalue_roll _returnvalue_pitch _returnvalue_yaw) (`KismetMathLibrary.BreakRotator` (`KismetMathLibrary.FindLookAtRotation` (`self.K2_GetActorLocation`) ActorLocation)))
  ;[1 0 0.04544] Add Hit Hunter
  (`parent.ApplyDamage` ActorLocation Value)
  (set `self.DamageElvenlin` true)
  (`/Engine/EditorBlueprintResources/StandardMacros.DoOnce` false :!label _label
    (:`Completed`
      (`PrimitiveComponent.SetCollisionProfileName` (`self.CapsuleComponent`) "Damage" true)
      (`MovementComponent.StopMovementImmediately` (`self.CharacterMovement`))
      (`self.StopJumping`)
      (set `self.isAttackElvenlin` false)
      (`self.DisableInput` null)
      (`|ExecutionSequence`
        (:`then_0`
          (if (== (`KismetMathLibrary.Abs` _returnvalue_yaw) 180.0)
            (`self.LaunchCharacter` (500.0 0.0 1000.0) false true)
            (set `self.isMoveRightElvenlin` false)
            (else
              (`self.LaunchCharacter` (-500.0 0.0 1000.0) false true)
              (set `self.isMoveRightElvenlin` true))))
        (:`then_1`
          (bind (_direction _color) (`Timeline|Timeline_0` :!via `PlayFromStart`)
            (:`Update`
              (`PaperFlipbookComponent.SetSpriteColor` (`self.Sprite`) _color))
            (:`Finished`
              (`PrimitiveComponent.SetCollisionProfileName` (`self.CapsuleComponent`) "Player" true)
              (set `self.DamageElvenlin` false)
              (`self.EnableInput` null)
              (goto _label :!via `Reset`))))))))

(event `InputAction|ChangePlayer`
  (params (Key :type "Key Structure"))
  ;[0.3798 1 0.9202] Change Player and possess
  (:`Pressed`
    (bind _outactors (`GameplayStatics.GetAllActorsOfClass` "/Game/PlayerHunter/BP_Hunter.BP_Hunter_C"))
    (for _array_element _outactors
      (`Controller.Possess` (`GameplayStatics.GetPlayerController` 0) _array_element)
      (bind _returnvalue (`GameplayStatics.GetActorOfClass` "/Game/Camera/BP_CameraAdvanced.BP_CameraAdvanced_C"))
      (message `/Game/Interfaces/I_Camera.SetNewPlayerFollow` _returnvalue _array_element))))

(event `self.ReceiveUnpossessed`
  (params (OldController :type "Controller Object Reference"))
  ;[0.3798 1 0.9202] Change Player and possess
  (`Controller.Possess` OldController self))

(event `self.OnLanded`
  (params (Hit :type "HitResult Structure (by ref)"))
  ;[1 0.02034 0.7621] Onlanded
  (`ParticleSystemComponent.SetTemplate` (`self.ParticleOnlanded`) "/Game/Particles/P_SmokeOnlanded.P_SmokeOnlanded"))

(event `self.TickedEvent`)

(fn `UserConstructionScript`)