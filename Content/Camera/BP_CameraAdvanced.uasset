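; Side-view camera actor that frames a followed actor on the X/Z plane at a set Y offset and rotation.
; SetActor places the camera at that actor's X and Z, running only on construction and BeginPlay.
; Events store X/Z zone limits, a Z dead zone and left/right direction, none of which this graph reads.
; SetNewPlayerFollow swaps the followed actor and makes this camera player 0's view target.
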(event `self.ReceiveBeginPlay`
  (`self.SetActor`))

(event `/Game/Interfaces/I_Camera.ZLimit`
  (params (MaxZ :type "Float (double-precision)") (MinZ :type "Float (double-precision)") (NewDeadZone :type "Float (double-precision)"))
  (set `self.MaxZoneZ` MaxZ)
  (set `self.MinZoneZ` MinZ)
  (set `self.DeadZoneZ` NewDeadZone))

(event `/Game/Interfaces/I_Camera.XLimit`
  (params (MaxX :type "Float (double-precision)") (MinX :type "Float (double-precision)"))
  (set `self.MaxZoneX` MaxX)
  (set `self.MinZoneX` MinX))

(event `/Game/Interfaces/I_Camera.DirectionActor`
  (params (LeftRightDirection :type Boolean))
  (set `self.LeftRight` LeftRightDirection))

(event `/Game/Interfaces/I_Camera.SetNewPlayerFollow`
  (params (Actor :type "Actor Object Reference"))
  (set `self.ActorFollow` Actor)
  (`PlayerController.SetViewTargetWithBlend` (`GameplayStatics.GetPlayerController` 0) self 0.0 "VTBlend_Linear" 0.0 false))

(fn `SetActor`
  (bind (_x _y _z) (`KismetMathLibrary.BreakVector3f` (`self.K2_GetActorLocation` (`self.ActorFollow`))))
  (`/Engine/EditorBlueprintResources/StandardMacros.IsValid` (`self.ActorFollow`)
    (:`Is Valid`
      (`SceneComponent.K2_SetRelativeLocationAndRotation` (`self.Camera`) (`KismetMathLibrary.MakeVector` _x (`self.OffsetCamera`) _z) (`self.RotationCameraYaw`) false false))))

(fn `UserConstructionScript`
  (`self.SetActor`))