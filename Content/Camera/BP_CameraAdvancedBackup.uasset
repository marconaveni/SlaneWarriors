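; Side-scrolling follow camera actor that becomes the first player's view target and tracks PlayerFollow at a fixed depth offset and rotation.
; A looping timer, rather than Tick, moves the camera component through MoveComponentTo, clamped to X and Z bounds.
; X gains a look-ahead offset that steps toward the direction set by DirectionActor, while Z uses a dead zone or fixed height.
; ZLimit and XLimit change the bounds at runtime.
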(event `self.ReceiveBeginPlay`
  (`PlayerController.SetViewTargetWithBlend` (`GameplayStatics.GetPlayerController` 0) self 0.0 "VTBlend_Linear" 0.0 false)
  (`KismetSystemLibrary.K2_SetTimerDelegate` (delegate `EventStart`) 0.016 true))

(event `EventStart`
  (bind _returnvalue_x (`KismetMathLibrary.BreakVector` (`self.K2_GetActorLocation` (`self.PlayerFollow`))))
  (`/Engine/EditorBlueprintResources/StandardMacros.IsValid` (`self.PlayerFollow`)
    (:`Is Valid`
      (bind _returnvalue (`self.XFollow`))
      (set `self.LeftRightOffset_0` _returnvalue)
      (bind _newzlocation (`self.ZFollow`))
      (set `self.FollowZ` (`KismetMathLibrary.FClamp` _newzlocation (`self.MinZoneZ_0`) (`self.MaxZoneZ_0`)))
      (`KismetSystemLibrary.MoveComponentTo` (`self.BCamera`) (`KismetMathLibrary.MakeVector` (`KismetMathLibrary.FClamp` (+ _returnvalue_x (`self.LeftRightOffset_0`)) (`self.MinZoneX_0`) (`self.MaxZoneX_0`)) (`self.OffsetCamera_0`) (`self.FollowZ`)) (`self.RotationCameraYaw_0`) false false (`self.Over Time`)))
    (:`Is Not Valid`
      (`KismetSystemLibrary.PrintString` "Error Select Actor to Follow Player" true true (struct :`R` 1.0 :`A` 1.0)))))

(event `self.ReceiveTick`
  (params (DeltaSeconds :type "Float (single-precision)")))

(event `/Game/Interfaces/I_Camera.ZLimit`
  (params (MaxZ :type "Float (double-precision)") (MinZ :type "Float (double-precision)") (NewDeadZone :type "Float (double-precision)"))
  (set `self.MaxZoneZ_0` MaxZ)
  (set `self.MinZoneZ_0` MinZ)
  (set `self.DeadZoneZ_0` NewDeadZone))

(event `/Game/Interfaces/I_Camera.XLimit`
  (params (MaxX :type "Float (double-precision)") (MinX :type "Float (double-precision)"))
  (set `self.MaxZoneX_0` MaxX)
  (set `self.MinZoneX_0` MinX))

(event `/Game/Interfaces/I_Camera.DirectionActor`
  (params (LeftRightDirection :type Boolean))
  (set `self.Left Right` LeftRightDirection))

(fn `DecreaseNumber`
  (params (Value :type "Float (double-precision)") (`-` :type "Float (double-precision)") (Min :type "Float (double-precision)") (Max :type "Float (double-precision)") (InclusiveMin :type Boolean) (InclusiveMax :type Boolean))
  (returns (ReturnValue :type "Float (double-precision)"))
  (if (`KismetMathLibrary.InRange_FloatFloat` Value Min Max InclusiveMin InclusiveMax)
    (return (- Value `-`))
    (else
      (return Value))))

(fn `IncreaseNumber`
  (params (Value :type "Float (double-precision)") (`+` :type "Float (double-precision)") (Min :type "Float (double-precision)") (Max :type "Float (double-precision)") (InclusiveMin :type Boolean) (InclusiveMax :type Boolean))
  (returns (ReturnValue :type "Float (double-precision)"))
  (if (`KismetMathLibrary.InRange_FloatFloat` Value Min Max InclusiveMin InclusiveMax)
    (return (+ Value `+`))
    (else
      (return Value))))

(fn `UserConstructionScript`
  (bind (_x _y _z) (`KismetMathLibrary.BreakVector3f` (`self.K2_GetActorLocation` (`self.PlayerFollow`))))
  (`/Engine/EditorBlueprintResources/StandardMacros.IsValid` (`self.PlayerFollow`)
    (:`Is Valid`
      (`self.K2_SetActorLocation` (0.0 0.0 0.0))
      (`SceneComponent.K2_SetRelativeLocationAndRotation` (`self.BCamera`) (`KismetMathLibrary.MakeVector` _x (`self.OffsetCamera_0`) _z) (`self.RotationCameraYaw_0`) false false))))

(fn `XFollow`
  (returns (ReturnValue :type "Float (double-precision)"))
  (if (`self.Left Right`)
    (return (`self.IncreaseNumber` (`self.LeftRightOffset_0`) 10.0 -400.0 400.0 true))
    (else
      (return (`self.DecreaseNumber` (`self.LeftRightOffset_0`) 10.0 -400.0 400.0 false true)))))

(fn `ZFollow`
  (returns (NewZLocation :type "Float (double-precision)"))
  (locals (ZFollowLocal :type "Float (double-precision)"))
  (bind (_returnvalue_x _returnvalue_y _returnvalue_z) (`KismetMathLibrary.BreakVector` (`self.K2_GetActorLocation`)))
  (bind (_returnvalue_x_2 _returnvalue_y_2 _returnvalue_z_2) (`KismetMathLibrary.BreakVector` (`self.K2_GetActorLocation`)))
  (bind (_returnvalue_x_3 _returnvalue_y_3 _returnvalue_z_3) (`KismetMathLibrary.BreakVector` (`self.K2_GetActorLocation` (`self.PlayerFollow`))))
  (bind (_returnvalue_x_4 _returnvalue_y_4 _returnvalue_z_4) (`KismetMathLibrary.BreakVector` (`self.K2_GetActorLocation` (`self.PlayerFollow`))))
  (bind _returnvalue (- _returnvalue_z_4 (`self.DeadZoneZ_0`)))
  (bind _returnvalue_2 (+ _returnvalue_z_3 (`self.DeadZoneZ_0`)))
  (if (!= (`self.FixedZoneZ`) 0.0)
    (return (`self.FixedZoneZ`))
    (elif (> _returnvalue _returnvalue_z_2)
      (return _returnvalue)
      (elif (< _returnvalue_2 _returnvalue_z)
        (return _returnvalue_2)))))