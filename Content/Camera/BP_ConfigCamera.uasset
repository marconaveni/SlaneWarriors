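; Camera configuration volume that sets movement limits and dead zone on the level's BP_CameraAdvanced while the player pawn is inside its Box.
; BeginPlay finds the camera and starts a looping 0.15-second timer that polls IsOverlapBox, leaving the component overlap event empty.
; While inside, each tick of the timer resends the X and Z limits and new dead zone.
; A local IsBoxOverlap function, testing only X and Z extents, is not called here.
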(event `self.Box.OnComponentBeginOverlap`
  (params (OverlappedComponent :type "PrimitiveComponent Object Reference") (OtherActor :type "Actor Object Reference") (OtherComp :type "PrimitiveComponent Object Reference") (OtherBodyIndex :type Integer) (bFromSweep :type Boolean) (SweepResult :type "HitResult Structure (by ref)")))

(event `self.ReceiveBeginPlay`
  (bind _returnvalue (`GameplayStatics.GetActorOfClass` "/Game/Camera/BP_CameraAdvanced.BP_CameraAdvanced_C"))
  (`/Engine/EditorBlueprintResources/StandardMacros.IsValid` _returnvalue
    (:`Is Valid`
      (set `self.BP Camera Advance` _returnvalue)
      (`KismetSystemLibrary.K2_SetTimerDelegate` (delegate `timer`) 0.15 true))))

(event `timer`
  (if (`SlaneFunctionLibrary.isOverlapBox` (`self.Box`) (`GameplayStatics.GetPlayerPawn` 0))
    (message `/Game/Interfaces/I_Camera.ZLimit` (`self.BP Camera Advance`) (`self.Max Z`) (`self.Min Z`) (`self.New Dead Zone`))
    (message `/Game/Interfaces/I_Camera.XLimit` (`self.BP Camera Advance`) (`self.Max X`) (`self.Min X`))))

(fn `isBoxOverlap`
  (returns (ReturnValue :type Boolean))
  (bind _returnvalue_x (`KismetMathLibrary.BreakVector` (`SceneComponent.K2_GetComponentLocation` (`self.Box`))))
  (bind _returnvalue_x_2 (`KismetMathLibrary.BreakVector` (`self.K2_GetActorLocation` (`GameplayStatics.GetPlayerPawn` 0))))
  (bind (_returnvalue_x_3 _returnvalue_y _returnvalue_z) (`KismetMathLibrary.BreakVector` (`SceneComponent.K2_GetComponentLocation` (`self.Box`))))
  (bind (_returnvalue_x_4 _returnvalue_y_2 _returnvalue_z_2) (`KismetMathLibrary.BreakVector` (`self.K2_GetActorLocation` (`GameplayStatics.GetPlayerPawn` 0))))
  (bind _boxextent_x (`KismetMathLibrary.BreakVector` (`BoxComponent.BoxExtent` (`self.Box`))))
  (bind (_boxextent_x_2 _boxextent_y _boxextent_z) (`KismetMathLibrary.BreakVector` (`BoxComponent.BoxExtent` (`self.Box`))))
  (bind _returnvalue (and (< (`KismetMathLibrary.Vector_Distance` (`KismetMathLibrary.MakeVector` _returnvalue_x) (`KismetMathLibrary.MakeVector` _returnvalue_x_2)) _boxextent_x) (< (`KismetMathLibrary.Vector_Distance` (`KismetMathLibrary.MakeVector` 0.0 0.0 _returnvalue_z) (`KismetMathLibrary.MakeVector` 0.0 0.0 _returnvalue_z_2)) _boxextent_z)))
  (if _returnvalue
    _
    (else
      _))
  (return _returnvalue))

(fn `UserConstructionScript`)