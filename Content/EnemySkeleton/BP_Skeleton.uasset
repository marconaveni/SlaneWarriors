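; Side-view skeleton enemy that patrols between X limits, reacts to and follows the player, and attacks with an axe.
; While alive, Tick drives movement, flipbook animations, box-based attack and follow checks, and footstep particle placement.
; The axe hitbox moves per attack frame, parks off-plane otherwise, and only damages during swing frames; body contact also hurts.
; Taking damage interrupts attacks with knockback and a color timeline, or plays death and disables collision.
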(event `Movement or set start attack`
  (bind _returnvalue_x (`KismetMathLibrary.BreakVector` (`self.K2_GetActorLocation`)))
  ;[0 0.01914 1] Movement or set start attack
  (`|ExecutionSequence`
    (:`then_0`
      (if (`SlaneFunctionLibrary.AnimationNotify` (`self.Sprite`) "/Game/EnemySkeleton/assets/React/Skeleton_React_.Skeleton_React_" 3)
        (set `self.React` false)))
    (:`then_1`
      (if (`self.IsAttack`)
        (if (and (`SlaneFunctionLibrary.AnimationNotify` (`self.Sprite`) "/Game/EnemySkeleton/assets/Attack/Skeleton_Attack_.Skeleton_Attack_" 6) (not (`SlaneFunctionLibrary.AnimationNotify` (`self.Sprite`) "/Game/EnemySkeleton/assets/Attack/Skeleton_Attack_.Skeleton_Attack_" 10)))
          (set `self.Hit` true)
          (else
            (set `self.Hit` false)))
        (elif (`self.DamageEnemy`)
          _
          (elif (`self.React`)
            (`SlaneFunctionLibrary.SetAnimation` (`self.Sprite`) "/Game/EnemySkeleton/assets/React/Skeleton_React_.Skeleton_React_")
            (else
              (`self.AddMovementInput` (1.0 0.0 0.0) (`self.Move`))
              (if (< _returnvalue_x (`self.MoveLeftLimit`))
                (set `self.Move` 1.0)
                (elif (> _returnvalue_x (`self.MoveRightLimit`))
                  (set `self.Move` -1.0))))))))))

(event `Set Hitbox Axe Default Location`
  ;[0.2628 1 0] Update position hitbox axe
  (set `self.HitboxAxeLocation` (0.0 1000.0 0.0))
  (`KismetSystemLibrary.MoveComponentTo` (`self.Hit box Axe`) (`self.HitboxAxeLocation`) (struct) false false 0.05 :!label _label))

(event `Set HitBox Axe Location Attack`
  ;[0.2628 1 0] Update position hitbox axe
  (switch `int` (`PaperFlipbookComponent.GetPlaybackPositionInFrames` (`self.Sprite`))
    (:`0`
      (set `self.HitboxAxeLocation` (0.0 1000.0 0.0))
      (goto _label))
    (:`1`
      (set `self.HitboxAxeLocation` (0.0 1000.0 0.0))
      (goto _label))
    (:`2`
      (set `self.HitboxAxeLocation` (0.0 1000.0 0.0))
      (goto _label))
    (:`3`
      (set `self.HitboxAxeLocation` (110.0 1000.0 150.0))
      (goto _label))
    (:`4`
      (set `self.HitboxAxeLocation` (-40.0 0.0 210.0))
      (goto _label))
    (:`5`
      (set `self.HitboxAxeLocation` (-80.0 0.0 210.0))
      (goto _label))
    (:`6`
      (set `self.HitboxAxeLocation` (-80.0 0.0 210.0))
      (goto _label))
    (:`7`
      (set `self.HitboxAxeLocation` (230.0 0.0 160.0))
      (goto _label))
    (:`8`
      (set `self.HitboxAxeLocation` (300.0 0.0 -110.0))
      (goto _label))
    (:`9`
      (set `self.HitboxAxeLocation` (290.0 0.0 -110.0))
      (goto _label))
    (:`10`
      (set `self.HitboxAxeLocation` (0.0 1000.0 0.0))
      (goto _label))
    (:`11`
      (set `self.HitboxAxeLocation` (0.0 1000.0 0.0))
      (goto _label))
    (:`12`
      (set `self.HitboxAxeLocation` (0.0 1000.0 0.0))
      (goto _label))
    (:`13`
      (set `self.HitboxAxeLocation` (0.0 1000.0 0.0))
      (goto _label))
    (:`14`
      (set `self.HitboxAxeLocation` (0.0 1000.0 0.0))
      (goto _label))
    (:`15`
      _)
    (:`16`
      _)
    (:`17`
      (set `self.HitboxAxeLocation` (0.0 1000.0 0.0))
      (goto _label)))
  (set `self.HitboxAxeLocation` (0.0 1000.0 0.0))
  (goto _label))

(event `self.ReceiveTick`
  (params (DeltaSeconds :type "Float (single-precision)"))
  ;[0.0926 1 0] Tick Events
  (if (> (`self.Life`) 0.0)
    (`self.Movement or set start attack`)
    (`self.UpdateAnimations`)
    (`self.Overlap Attack Collision`)
    (`self.Follow Player`)
    (`self.FootStep`)))

(event `UpdateAnimations`
  (bind _velocity_x (`KismetMathLibrary.BreakVector` (`MovementComponent.Velocity` (`self.CharacterMovement`))))
  ;[0 0.9085 1] Animations
  (if (or (`self.DamageEnemy`) (`self.React`))
    (`self.Set Hitbox Axe Default Location`)
    (elif (`self.IsAttack`)
      (`SlaneFunctionLibrary.SetAnimation` (`self.Sprite`) "/Game/EnemySkeleton/assets/Attack/Skeleton_Attack_.Skeleton_Attack_" true)
      (`self.Set HitBox Axe Location Attack`)
      (elif (!= _velocity_x 0.0)
        (`SlaneFunctionLibrary.SetAnimation` (`self.Sprite`) "/Game/EnemySkeleton/assets/Walk/Skeleton_Walk_.Skeleton_Walk_" true)
        (`self.Set Hitbox Axe Default Location`)
        (else
          (`SlaneFunctionLibrary.SetAnimation` (`self.Sprite`) "/Game/EnemySkeleton/assets/idle/Skeleton_Idle_.Skeleton_Idle_" true)
          (`self.Set Hitbox Axe Default Location`))))))

(event `Overlap Attack Collision`
  ;[1 0.01025 0.9943] Set Attack if overlap with box collision "Attack Collision"
  (if (or (`SlaneFunctionLibrary.AnimationNotify` (`self.Sprite`) "/Game/EnemySkeleton/assets/Attack/Skeleton_Attack_.Skeleton_Attack_" 16) (not (`self.IsAttack`)))
    (set `self.IsAttack` (`SlaneFunctionLibrary.isOverlapBox` (`self.AttackCollision`) (`self.ActorAttack`)))))

(event `Follow Player`
  (bind (_returnvalue_roll _returnvalue_pitch _returnvalue_yaw) (`KismetMathLibrary.BreakRotator` (`self.K2_GetActorRotation`)))
  (bind (_returnvalue_roll_2 _returnvalue_pitch_2 _returnvalue_yaw_2) (`KismetMathLibrary.BreakRotator` (`KismetMathLibrary.FindLookAtRotation` (`self.K2_GetActorLocation`) (`self.K2_GetActorLocation` (`self.ActorAttack`)))))
  ;[0 0.2305 1] Follow Player
  (if (`SlaneFunctionLibrary.isOverlapBox` (`self.FollowCollision`) (`self.ActorAttack`))
    (if (not (`SlaneFunctionLibrary.AnimationNotify` (`self.Sprite`) "/Game/EnemySkeleton/assets/Attack/Skeleton_Attack_.Skeleton_Attack_" 3))
      (`self.K2_SetActorRotation` (`KismetMathLibrary.MakeRotator` 0.0 0.0 _returnvalue_yaw_2))
      (if (< _returnvalue_yaw 180.0)
        (set `self.Move` 1.0)
        (else
          (set `self.Move` -1.0))))))

(event `self.ApplyDamageEnemy`
  (params (ActorLocation :type "Vector Structure") (Value :type "Float (single-precision)"))
  (bind _life (`self.Life`))
  (bind (_returnvalue_roll _returnvalue_pitch _returnvalue_yaw) (`KismetMathLibrary.BreakRotator` (`KismetMathLibrary.FindLookAtRotation` (`self.K2_GetActorLocation`) ActorLocation)))
  ;[1 0 0.04519] Receiver Damage Enemy
  (set `self.ActorAttack` (`GameplayStatics.GetPlayerPawn` 0))
  (set `self.DamageEnemy` true)
  (set `self.IsAttack` false)
  (`MovementComponent.StopMovementImmediately` (`self.CharacterMovement`))
  (set `self.Life` (- (`self.Life`) Value))
  (`KismetSystemLibrary.PrintString` (`KismetStringLibrary.Conv_DoubleToString` _life))
  (if (<= _life 0.0)
    (`SlaneFunctionLibrary.SetAnimation` (`self.Sprite`) "/Game/EnemySkeleton/assets/Skeleton_Dead_.Skeleton_Dead_")
    (`self.SetActorEnableCollision` false)
    (else
      (`SlaneFunctionLibrary.SetAnimation` (`self.Sprite`) "/Game/EnemySkeleton/assets/Hit/Skeleton_Hit_.Skeleton_Hit_" false true)
      (`|ExecutionSequence`
        (:`then_0`
          (if (== _returnvalue_yaw 180.0)
            (`self.LaunchCharacter` (700.0 0.0 0.0) false true)
            (else
              (`self.LaunchCharacter` (-700.0 0.0 0.0) false true))))
        (:`then_1`
          (bind (_direction _color) (`Timeline|Timeline_1` :!via `PlayFromStart`)
            (:`Update`
              (`PaperFlipbookComponent.SetSpriteColor` (`self.Sprite`) _color))
            (:`Finished`
              (set `self.DamageEnemy` false)
              (set `self.React` false))))))))

(event `Hit Event`
  ;[1 0.7569 0] Apply Damage Player
)

(event `self.Hit box Axe.OnComponentBeginOverlap`
  (params (OverlappedComponent :type "PrimitiveComponent Object Reference") (OtherActor :type "Actor Object Reference") (OtherComp :type "PrimitiveComponent Object Reference") (OtherBodyIndex :type Integer) (bFromSweep :type Boolean) (SweepResult :type "HitResult Structure (by ref)"))
  ;[1 0.7569 0] Apply Damage Player
  (if (`self.Hit`)
    (bind _asplayer_character (cast `PlayerCharacter` OtherActor))
    (`InteractInterface.ApplyDamage` _asplayer_character (`self.K2_GetActorLocation`) 1.0)
    (set `self.ActorAttack` _asplayer_character)
    (bind _outactors (`GameplayStatics.GetAllActorsOfClass` "/Script/SlaneWarriors.EnemyCharacter"))
    (bind _outhit (`KismetSystemLibrary.LineTraceSingle` (`self.K2_GetActorLocation`) (`SceneComponent.K2_GetComponentLocation` (`self.Hit box Axe`)) "TraceTypeQuery1" false _outactors "None" true (struct :`R` 1.0 :`A` 1.0) (struct :`G` 1.0 :`A` 1.0) 3.0))
    (bind (_x _y _z) (`KismetMathLibrary.BreakVector3f` (`.TraceEnd` (`GameplayStatics.BreakHitResult` _outhit))))
    (`SceneComponent.K2_SetWorldLocation` (`self.SpriteParticle`) (`KismetMathLibrary.MakeVector` _x (+ _y 10.0) _z) false false)
    (`SlaneFunctionLibrary.SetAnimation` (`self.SpriteParticle`) "/Game/Effects/Effect_Hit.Effect_Hit" false true)))

(event `self.CapsuleComponent.OnComponentBeginOverlap`
  (params (OverlappedComponent :type "PrimitiveComponent Object Reference") (OtherActor :type "Actor Object Reference") (OtherComp :type "PrimitiveComponent Object Reference") (OtherBodyIndex :type Integer) (bFromSweep :type Boolean) (SweepResult :type "HitResult Structure (by ref)"))
  ;[1 0.7569 0] Apply Damage Player
  (bind _asplayer_character (cast `PlayerCharacter` OtherActor))
  (if (== (`Character.CapsuleComponent` _asplayer_character) OtherComp)
    (`InteractInterface.ApplyDamage` _asplayer_character (`self.K2_GetActorLocation`) 1.0)))

(event `FootStep`
  (bind (_returnvalue_x _returnvalue_y _returnvalue_z) (`KismetMathLibrary.BreakVector` (`self.K2_GetActorLocation`)))
  (bind (_returnvalue_x_2 _returnvalue_y_2 _returnvalue_z_2) (`KismetMathLibrary.BreakVector` (`self.K2_GetActorLocation`)))
  (bind _velocity_x (`KismetMathLibrary.BreakVector` (`MovementComponent.Velocity` (`self.CharacterMovement`))))
  ;[0.1058 0 1] Particles
  (if (and (!= _velocity_x 0.0) (not (`NavMovementComponent.IsFalling` (`self.CharacterMovement`))))
    (`SceneComponent.K2_SetWorldLocation` (`self.ParticleFootStep`) (`KismetMathLibrary.MakeVector` _returnvalue_x (- _returnvalue_y 1.0) (- _returnvalue_z 108.0)) false false)
    (else
      (`SceneComponent.K2_SetWorldLocation` (`self.ParticleFootStep`) (`KismetMathLibrary.MakeVector` _returnvalue_x_2 (- _returnvalue_y_2 50.0) (- _returnvalue_z_2 108.0)) false false))))

(event `self.AttackCollision.OnComponentBeginOverlap`
  (params (OverlappedComponent :type "PrimitiveComponent Object Reference") (OtherActor :type "Actor Object Reference") (OtherComp :type "PrimitiveComponent Object Reference") (OtherBodyIndex :type Integer) (bFromSweep :type Boolean) (SweepResult :type "HitResult Structure (by ref)"))
  (bind _asplayer_character (cast `PlayerCharacter` OtherActor))
  (set `self.ActorAttack` _asplayer_character))

(event `self.ReceiveBeginPlay`
  (set `self.ActorAttack` (`GameplayStatics.GetPlayerPawn` 0)))

(event `self.FollowCollision.OnComponentBeginOverlap`
  (params (OverlappedComponent :type "PrimitiveComponent Object Reference") (OtherActor :type "Actor Object Reference") (OtherComp :type "PrimitiveComponent Object Reference") (OtherBodyIndex :type Integer) (bFromSweep :type Boolean) (SweepResult :type "HitResult Structure (by ref)"))
  (bind _asplayer_character (cast `PlayerCharacter` OtherActor))
  (set `self.ActorAttack` _asplayer_character)
  (set `self.React` true))

(fn `bis box Overlap `
  (params (`Box Collision` :type "BoxComponent Object Reference") (Ator :type "Actor Object Reference"))
  (returns (Output :type Boolean))
  (bind _returnvalue_x (`KismetMathLibrary.BreakVector` (`SceneComponent.K2_GetComponentLocation` `Box Collision`)))
  (bind _returnvalue_x_2 (`KismetMathLibrary.BreakVector` (`self.K2_GetActorLocation` Ator)))
  (bind (_returnvalue_x_3 _returnvalue_y _returnvalue_z) (`KismetMathLibrary.BreakVector` (`SceneComponent.K2_GetComponentLocation` `Box Collision`)))
  (bind (_returnvalue_x_4 _returnvalue_y_2 _returnvalue_z_2) (`KismetMathLibrary.BreakVector` (`self.K2_GetActorLocation` Ator)))
  (bind _boxextent_x (`KismetMathLibrary.BreakVector` (`BoxComponent.BoxExtent` `Box Collision`)))
  (bind (_boxextent_x_2 _boxextent_y _boxextent_z) (`KismetMathLibrary.BreakVector` (`BoxComponent.BoxExtent` `Box Collision`)))
  (return (and (< (`KismetMathLibrary.Vector_Distance` (`KismetMathLibrary.MakeVector` _returnvalue_x) (`KismetMathLibrary.MakeVector` _returnvalue_x_2)) _boxextent_x) (< (`KismetMathLibrary.Vector_Distance` (`KismetMathLibrary.MakeVector` 0.0 0.0 _returnvalue_z) (`KismetMathLibrary.MakeVector` 0.0 0.0 _returnvalue_z_2)) _boxextent_z))))

(fn `UserConstructionScript`)