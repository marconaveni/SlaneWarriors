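; Parallax background actor that moves three tile map layers along with a BP_CameraAdvanced camera to create depth.
; Construction and BeginPlay assign the tile maps; BeginPlay also caches the CameraFollow camera and offsets the root along Y by DistanceParallax.
; A fast looping timer, used instead of Tick, repositions each layer in X and Z from the camera component's relative location, using per-layer offsets and follow factors.
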(event `self.ReceiveBeginPlay`
  (bind (_relativelocation_x _relativelocation_y _relativelocation_z) (`KismetMathLibrary.BreakVector` (`SceneComponent.RelativeLocation` (`self.DefaultSceneRoot`))))
  (bind _asbp_camera_advanced (cast `/Game/Camera/BP_CameraAdvanced` (`self.CameraFollow`)))
  (set `self.BP Camera Advanced` _asbp_camera_advanced)
  (`PaperTileMapComponent.SetTileMap` (`self.Layer1`) (`self.New Tile Map0`))
  (`PaperTileMapComponent.SetTileMap` (`self.Layer2`) (`self.New Tile Map1`))
  (`PaperTileMapComponent.SetTileMap` (`self.Layer3`) (`self.New Tile Map2`))
  (`SceneComponent.K2_SetRelativeLocation` (`self.DefaultSceneRoot`) (`KismetMathLibrary.MakeVector` _relativelocation_x (- _relativelocation_y (`self.Distance Parallax`)) _relativelocation_z) false false)
  (`KismetSystemLibrary.K2_SetTimerDelegate` (delegate `tick custom`) 0.008 true))

(event `tick custom`
  (bind (_camera_location_x _camera_location_y _camera_location_z) (`KismetMathLibrary.BreakVector` (`self.Camera Location`)))
  (bind (_camera_location_x_2 _camera_location_y_2 _camera_location_z_2) (`KismetMathLibrary.BreakVector` (`self.Camera Location`)))
  (bind (_camera_location_x_3 _camera_location_y_3 _camera_location_z_3) (`KismetMathLibrary.BreakVector` (`self.Camera Location`)))
  (bind (_returnvalue_x _returnvalue_y) (`KismetMathLibrary.BreakVector` (`SceneComponent.K2_GetComponentLocation` (`self.Layer3`))))
  (bind (_returnvalue_x_2 _returnvalue_y_2) (`KismetMathLibrary.BreakVector` (`SceneComponent.K2_GetComponentLocation` (`self.Layer1`))))
  (bind (_returnvalue_x_3 _returnvalue_y_3) (`KismetMathLibrary.BreakVector` (`SceneComponent.K2_GetComponentLocation` (`self.Layer2`))))
  (bind _returnvalue_location (`KismetMathLibrary.BreakTransform` (`SceneComponent.GetRelativeTransform` (`CameraSideScroller.Camera` (`self.BP Camera Advanced`)))))
  (`/Engine/EditorBlueprintResources/StandardMacros.IsValid` (`self.BP Camera Advanced`)
    (:`Is Valid`
      (set `self.Camera Location` _returnvalue_location)
      (`SceneComponent.K2_SetWorldLocation` (`self.Layer1`) (`KismetMathLibrary.MakeVector` (* (- _camera_location_x 4500.0) 0.95) _returnvalue_y_2 (* (- _camera_location_z -2900.0) 0.98)) false false)
      (`SceneComponent.K2_SetWorldLocation` (`self.Layer2`) (`KismetMathLibrary.MakeVector` (* (- _camera_location_x_2 4500.0) 0.85) _returnvalue_y_3 (* (- _camera_location_z_2 -3500.0) 0.8)) false false)
      (`SceneComponent.K2_SetWorldLocation` (`self.Layer3`) (`KismetMathLibrary.MakeVector` (* (- _camera_location_x_3 4400.0) 0.7) _returnvalue_y (* (- _camera_location_z_3 -4900.0) 0.6)) false false))
    (:`Is Not Valid`
      (`KismetSystemLibrary.PrintString` "erro"))))

(event `self.ReceiveTick`
  (params (DeltaSeconds :type "Float (single-precision)")))

(fn `UserConstructionScript`
  (`PaperTileMapComponent.SetTileMap` (`self.Layer1`) (`self.New Tile Map0`))
  (`PaperTileMapComponent.SetTileMap` (`self.Layer2`) (`self.New Tile Map1`))
  (`PaperTileMapComponent.SetTileMap` (`self.Layer3`) (`self.New Tile Map2`)))