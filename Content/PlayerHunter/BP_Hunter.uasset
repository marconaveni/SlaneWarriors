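; Player-controlled Hunter character for a side-scrolling game with sprite visuals, dash, coyote jump and switching possession to BP_Elvenlin.
; Damage is gated by a DoOnce, locks input, applies knockback and a timeline color flash, then resets, or disables collision at zero life.
; Dash uses a timeline to ramp speed with gravity off, while coyote jump extends CanJumpInternal with a short falling timer.
; Movement and player switching notify BP_CameraAdvanced, and attack hits play a sprite effect.
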(event `self.TickedEvent`
  ;[0 1 0.2238] Tick - Updates animation
  (`|ExecutionSequence`))

(event `InputAction|Attack` :overrideparent false
  (params (Key :type "Key Structure")))

(event `self.AttackHitResult`
  (params (OutHit :type "HitResult Structure"))
  (bind (_x _y _z) (`KismetMathLibrary.BreakVector3f` (`.Location` (`GameplayStatics.BreakHitResult` OutHit))))
  ;[1 1 1] Comment
  (`SceneComponent.K2_SetWorldLocation` (`self.SpriteParticle`) (`KismetMathLibrary.MakeVector` _x (+ _y 10.0) _z) false false)
  (`SlaneFunctionLibrary.SetAnimation` (`self.SpriteParticle`) "/Game/Effects/Effect_Hit.Effect_Hit" false true))

(event `self.ApplyDamageCharacter`
  (params (ActorLocation :type "Vector Structure") (Value :type "Float (single-precision)"))
  (bind (_returnvalue_roll _returnvalue_pitch _returnvalue_yaw) (`KismetMathLibrary.BreakRotator` (`KismetMathLibrary.FindLookAtRotation` (`self.K2_GetActorLocation`) ActorLocation)))
  ;[1 0 0.04544] Receiver Damage Hunter
  (`KismetSystemLibrary.PrintString` "bp aconteceu")
  (set `self.DamageHunter` true)
  (`/Engine/EditorBlueprintResources/StandardMacros.DoOnce` false :!label _label
    (:`Completed`
      (`PrimitiveComponent.SetCollisionProfileName` (`self.CapsuleComponent`) "Damage" true)
      (`MovementComponent.StopMovementImmediately` (`self.CharacterMovement`))
      (`self.StopJumping`)
      (set `self.isAttack` false)
      (set `self.CountAttack` 0)
      (`self.DisableInput` null)
      (set `self.Life` (- (`self.Life`) Value))
      (if (> (`self.Life`) 0.0)
        (`|ExecutionSequence`
          (:`then_0`
            (if (== (`KismetMathLibrary.Abs` _returnvalue_yaw) 180.0)
              (`self.LaunchCharacter` (500.0 0.0 1000.0) false true)
              (set `self.isMoveRight` false)
              (else
                (`self.LaunchCharacter` (-500.0 0.0 1000.0) false true)
                (set `self.isMoveRight` true))))
          (:`then_1`
            (bind (_direction _color) (`Timeline|TimeColor` :!via `PlayFromStart`)
              (:`Update`
                (`PaperFlipbookComponent.SetSpriteColor` (`self.Sprite`) _color))
              (:`Finished`
                (`PrimitiveComponent.SetCollisionProfileName` (`self.CapsuleComponent`) "Player" true)
                (set `self.DamageHunter` false)
                (`self.EnableInput` null)
                (`self.ResetReceiverDamageHunter`)))))
        (else
          (`self.SetActorEnableCollision` false))))))

(event `ResetReceiverDamageHunter`
  ;[1 0 0.04544] Receiver Damage Hunter
  (goto _label :!via `Reset`))

(event `InputAxis|MoveRight` :overrideparent false
  (params (AxisValue :type "Float (single-precision)"))
  (bind _velocity_x (`KismetMathLibrary.BreakVector` (`MovementComponent.Velocity` (`self.CharacterMovement`))))
  (bind _velocity_x_2 (`KismetMathLibrary.BreakVector` (`MovementComponent.Velocity` (`self.CharacterMovement`))))
  ;[1 0.1765 0.1451] Handle movement
  (if (not (`self.isAttack`))
    (`/Engine/EditorBlueprintResources/StandardMacros.CompareFloat` AxisValue
      (:`>`
        (if (> _velocity_x_2 200.0)
          (bind _returnvalue (`GameplayStatics.GetActorOfClass` "/Game/Camera/BP_CameraAdvanced.BP_CameraAdvanced_C"))
          (message `/Game/Interfaces/I_Camera.DirectionActor` _returnvalue (`self.isMoveRight`))))
      (:`<`
        (if (< _velocity_x -200.0)
          (bind _returnvalue_2 (`GameplayStatics.GetActorOfClass` "/Game/Camera/BP_CameraAdvanced.BP_CameraAdvanced_C"))
          (message `/Game/Interfaces/I_Camera.DirectionActor` _returnvalue_2 (`self.isMoveRight`)))))))

(event `InputAction|Dash`
  (params (Key :type "Key Structure"))
  (bind _charactermovement (`self.CharacterMovement`))
  ;[1 0.1765 0.1451] Dash
  (:`Pressed`
    (`self.DisableInput` null)
    (`KismetSystemLibrary.Delay` 0.05)
    (set `self.isDash` true)
    (`MovementComponent.StopMovementImmediately` _charactermovement)
    (set `CharacterMovementComponent.GravityScale` 0.0 _charactermovement)
    (bind (_direction _slide_value) (`Timeline|Dash Time` :!via `PlayFromStart`)
      (:`Update`
        (set `CharacterMovementComponent.MaxWalkSpeed` (`KismetMathLibrary.Lerp` 0.0 3000.0 _slide_value) (`self.CharacterMovement`))
        (set `CharacterMovementComponent.MaxAcceleration` 20000.0 (`self.CharacterMovement`))
        (if (`self.isMoveRight`)
          (`self.AddMovementInput` (1.0 0.0 0.0))
          (else
            (`self.AddMovementInput` (1.0 0.0 0.0) -1.0))))
      (:`Finished`
        (set `CharacterMovementComponent.MaxWalkSpeed` 900.0 (`self.CharacterMovement`))
        (set `CharacterMovementComponent.MaxAcceleration` 2048.0 (`self.CharacterMovement`))
        (`MovementComponent.StopMovementImmediately` (`self.CharacterMovement`))
        (set `CharacterMovementComponent.GravityScale` 4.5 (`self.CharacterMovement`))
        (set `self.isDash` false)
        (set `self.isAttack` false)
        (set `self.CountAttack` 0)
        (set `self.isOnLandedAnimation` false)
        (`self.EnableInput` null)))))

(event `self.K2_OnMovementModeChanged`
  (params (PrevMovementMode :type "EMovementMode Enum" :default "MOVE_None") (NewMovementMode :type "EMovementMode Enum" :default "MOVE_None") (PrevCustomMode :type Byte) (NewCustomMode :type Byte))
  ;[0.2682 0 1] Coyote Jump
  (if (`|EnumEquality` NewMovementMode "MOVE_Falling")
    (bind _returnvalue (`KismetSystemLibrary.K2_SetTimerDelegate` (delegate `CoyoteJump`) 0.2))
    (set `self.Timer` _returnvalue)))

(event `InputAction|ChangePlayer`
  (params (Key :type "Key Structure"))
  ;[0.3798 1 0.9202] Change Player and possess
  (:`Pressed`
    (bind _outactors (`GameplayStatics.GetAllActorsOfClass` "/Game/PlayerElvenlin/BP_Elvenlin.BP_Elvenlin_C"))
    (for _array_element _outactors
      (`Controller.Possess` (`GameplayStatics.GetPlayerController` 0) _array_element)
      (bind _returnvalue (`GameplayStatics.GetActorOfClass` "/Game/Camera/BP_CameraAdvanced.BP_CameraAdvanced_C"))
      (message `/Game/Interfaces/I_Camera.SetNewPlayerFollow` _returnvalue _array_element))))

(event `CoyoteJump`
  ;[0.2682 0 1] Coyote Jump
)

(event `self.ReceiveUnpossessed`
  (params (OldController :type "Controller Object Reference"))
  ;[0.3798 1 0.9202] Change Player and possess
  (`Controller.Possess` OldController self))

(event `self.OnLanded`
  (params (Hit :type "HitResult Structure (by ref)"))
  ;[1 0 0.2259] OnLanded
  (`KismetSystemLibrary.K2_ClearAndInvalidateTimerHandle` (`self.Timer`))
  (`ParticleSystemComponent.SetTemplate` (`self.ParticleOnlanded`) "/Game/Particles/P_SmokeOnlanded.P_SmokeOnlanded"))

(fn `CanJumpInternal`
  (returns (ReturnValue :type Boolean))
  (bind _returnvalue (`parent.CanJumpInternal`))
  (return (or _returnvalue (> (`KismetSystemLibrary.K2_GetTimerRemainingTimeHandle` (`self.Timer`)) 0.0))))

(fn `UserConstructionScript`)